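; Test snowboard Blueprint in the skateboard system that lets the player fire off the item it is holding.
; On the ActivateItem press, it gets the held item class from ItemController and always spawns it at the mesh's world transform.
; It then passes that actor back to ItemController for activation, flagged as not held, with a position a fixed distance ahead.
; The construction script only calls the parent, and the other events are disabled stubs.
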(event EventBeginPlay
  (|CallParentFunction) ; This node is disabled and will not be called.\nDrag off pins to build functionality.
)

(event Collision|EventActorBeginOverlap
  (params (OtherActor :type Actor%20Object%20Reference)))

(event EventTick
  (params (DeltaSeconds :type Float%20%28single-precision%29))
  (|CallParentFunction DeltaSeconds) ; This node is disabled and will not be called.\nDrag off pins to build functionality.
)

(event Input|ActionEvents|InputActionActivateItem
  (params (Key :type Key%20Structure :default "None"))
  ;[0.6282 1 0.9299] Item Activation Handler
  (:Pressed
    (bind _returnvalue (Class|ItemController|GetHeldItem (Variables|Default|GetItemController)))
    (bind _returnvalue_2 (Game|SpawnActorfromClass _returnvalue (Transformation|GetWorldTransform (Variables|Character|GetMesh)) "AlwaysSpawn" 0 0))
    (Class|ItemController|ActivateHeldItem (Variables|Default|GetItemController) (+ (* (Transformation|GetActorForwardVector) 5e+02) (Transformation|GetActorLocation)) _returnvalue_2 false)))

(fn ConstructionScript
  (|CallParentFunction))